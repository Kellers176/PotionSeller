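; Potion-shop customer NPC that greets the player on overlap and orders a random potion through floating text.
; An overlapping item whose root component tag matches the order is destroyed and thanked; otherwise the order is repeated.
; After thanks, the NPC walks to a tagged walk-away point and back to order again.
; Tick, gated by a one-second Delay, drives movement, player-facing rotation and a debug-printed countdown whose time-out message is unreachable.
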(event `self.ReceiveBeginPlay`
  (bind _outactors (`GameplayStatics.GetAllActorsWithTag` "CustomerWalkAwayPoint"))
  (set `self.MoveToPoint` (`|GetArrayItem` _outactors))
  ;[1 1 1] Make clear at beginning of game - Collapsed into contained Macro
  (`SceneComponent.SetVisibility` (`self.RenderBackground`) false false)
  (bind _output_get (set `self.HeyText` ""))
  (`TextRenderComponent.K2_SetText` (`self.TextRender`) _output_get))

(event `self.ReceiveActorBeginOverlap`
  (params (OtherActor :type "Actor Object Reference"))
  (bind _targetpotion (`self.TargetPotion`))
  (bind _playerintrigger (`self.PlayerInTrigger`))
  (bind _rootcomponent (`Actor.RootComponent` OtherActor))
  (if (`self.ActorHasTag` OtherActor "Player")
    (set `self.PlayerInTrigger` true)
    ;[1 1 1] Setting the background to appear as well
    (`SceneComponent.SetVisibility` (`self.RenderBackground`) true false)
    (if (`self.PotionDecided`)
      (bind _output_get (set `self.HeyText` (`KismetTextLibrary.Conv_StringToText` (`self.FinalSaying`)) :!label _label))
      (`TextRenderComponent.K2_SetText` (`self.TextRender`) _output_get)
      (else
        (set `self.PotionDecided` true)
        (bind _output_get_2 (set `self.HeyText` "Potion Seller!"))
        (`TextRenderComponent.K2_SetText` (`self.TextRender`) _output_get_2)
        (`KismetSystemLibrary.Delay` 1.0)
        (if _playerintrigger
          (bind _output_get_3 (set `self.HeyText` "I require your strongest potion!"))
          (`TextRenderComponent.K2_SetText` (`self.TextRender`) _output_get_3)
          (`KismetSystemLibrary.Delay` 1.0))
        (`self.SetPotion` _playerintrigger)
        (set `self.minutes` 1.0)
        (set `self.seconds` 59.0)))
    (elif (not (`self.ActorHasTag` OtherActor "Customer"))
      (`KismetSystemLibrary.PrintString` _targetpotion)
      (`KismetSystemLibrary.PrintString` _rootcomponent (`KismetSystemLibrary.GetDisplayName` _rootcomponent))
      (if (`ActorComponent.ComponentHasTag` _rootcomponent (`KismetStringLibrary.Conv_StringToName` _targetpotion))
        ;[1 1 1] Correct Potion given to the customer
        (`self.K2_DestroyActor` OtherActor)
        (`SceneComponent.SetVisibility` (`self.RenderBackground`) true false)
        (bind _output_get_4 (set `self.HeyText` "Yes! Thank you potion seller!"))
        (`TextRenderComponent.K2_SetText` (`self.TextRender`) _output_get_4)
        (set `self.StillThanking` true)
        (`KismetSystemLibrary.Delay` 2.0)
        (set `self.StillThanking` false)
        (set `self.PotionDecided` false)
        (`self.SetTextToClear`
          (:`NewParam2`
            (set `self.NPCWalkingAway` true)))
        (else
          (`SceneComponent.SetVisibility` (`self.RenderBackground`) true false)
          (goto _label))))))

(event `self.ReceiveActorEndOverlap`
  (params (OtherActor :type "Actor Object Reference"))
  ;[1 1 1] Make clear when player is not near
  (set `self.PlayerInTrigger` false)
  (`self.SetTextToClear`))

(event `self.ReceiveTick`
  (params (DeltaSeconds :type "Float (single-precision)"))
  (`KismetSystemLibrary.Delay` 1.0)
  (`self.DecreaseTimer`)
  (`KismetSystemLibrary.PrintString` (`KismetStringLibrary.Concat_StrStr` (`KismetStringLibrary.Conv_DoubleToString` (`self.minutes`)) (`KismetStringLibrary.Conv_DoubleToString` (`self.seconds`))))
  (if (`self.NPCWalkingAway`)
    (if (`self.CustomerReturning`)
      (`self.ReturnToOrder`)
      (else
        (`self.WalkAway`)))
    (else
      ;[1 1 1] Make the NPC face the player
      (`SceneComponent.K2_SetWorldRotation` (`self.DefaultSceneRoot`) (`KismetMathLibrary.MakeRotator` 0.0 0.0 (.yaw (`KismetMathLibrary.FindLookAtRotation` (`self.K2_GetActorLocation`) (`self.K2_GetActorLocation` (`GameplayStatics.GetPlayerCharacter` 0))))) false false))))

(fn `CheckPotionIsRight`
  (params (Actor :type "Actor Object Reference")))

(fn `DecreaseTimer`
  (set `self.seconds` (- (`self.seconds`) 1.0))
  (if (< (`self.seconds`) 0.0)
    (set `self.minutes` (- (`self.minutes`) 1.0))
    (set `self.seconds` 59.0)
    (if (== (`self.seconds`) 0.0)
      (if (== (`self.minutes`) 0.0)
        (`KismetSystemLibrary.PrintString` "You ran out of time")))))

(fn `ReturnToOrder`
  (`self.K2_SetActorTransform` (`KismetMathLibrary.MakeTransform` (+ (* (`KismetMathLibrary.Normal` (`KismetMathLibrary.GetDirectionUnitVector` (`self.K2_GetActorLocation` self) (`self.CustomerOrderPoint`))) (* (`GameplayStatics.GetWorldDeltaSeconds`) (`self.NPCWalkSpeed`))) (.location (`self.GetTransform`))) (.rotation (`self.GetTransform`)) (.scale (`self.GetTransform`))))
  (if (< (`KismetMathLibrary.Abs` (/ (+ (.x (- (`self.K2_GetActorLocation` self) (`self.CustomerOrderPoint`))) (.y (- (`self.K2_GetActorLocation` self) (`self.CustomerOrderPoint`))) (.z (- (`self.K2_GetActorLocation` self) (`self.CustomerOrderPoint`)))) 3.0)) 0.5)
    (set `self.NPCWalkingAway` false)
    (set `self.CustomerReturning` false)))

(fn `SetPotion`
  (params (shouldDisplay :type Boolean))
  (bind _output_get (set `self.HeyText` "Make me a "))
  (set `self.TargetPotion` (`|GetArrayItem` (`self.PotionNames`) (`KismetMathLibrary.RandomInteger` 3)))
  (bind _output_get_2 (set `self.HeyText` (`KismetTextLibrary.Conv_StringToText` (`KismetStringLibrary.Concat_StrStr` (`KismetTextLibrary.Conv_TextToString` _output_get) (`KismetStringLibrary.Concat_StrStr` (`self.TargetPotion`) " potion!")))))
  (set `self.FinalSaying` (`KismetTextLibrary.Conv_TextToString` _output_get_2))
  (if shouldDisplay
    (`TextRenderComponent.K2_SetText` (`self.TextRender`) _output_get_2)
    (else
      (bind _output_get_3 (set `self.HeyText` ""))
      (`TextRenderComponent.K2_SetText` (`self.TextRender`) _output_get_3))))

(fn `UserConstructionScript`)

(fn `WalkAway`
  (locals (HasPointToMoveTo :type Boolean))
  (bind _returnvalue (< (`self.GetDistanceTo` self (`self.MoveToPoint`)) 2.0))
  (`self.K2_SetActorTransform` (`KismetMathLibrary.MakeTransform` (+ (* (`KismetMathLibrary.Normal` (`KismetMathLibrary.GetDirectionUnitVector` (`self.K2_GetActorLocation` self) (`self.K2_GetActorLocation` (`self.MoveToPoint`)))) (* (`GameplayStatics.GetWorldDeltaSeconds`) (`self.NPCWalkSpeed`))) (.location (`self.GetTransform`))) (.rotation (`self.GetTransform`)) (.scale (`self.GetTransform`))))
  (if _returnvalue
    _
    (else
      _))
  (set `self.CustomerReturning` _returnvalue))