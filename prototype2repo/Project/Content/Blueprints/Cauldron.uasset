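; Cauldron actor that consumes ingredient Items dropped into its Pit and brews potions from a list of recipes.
; Overlapping Items tagged Ingredient are counted by name in an Inventory map and destroyed, then every recipe is checked.
; Matching tests only that each ingredient type is present, ignoring quantity.
; A match spawns the recipe's output at SpawnLocation with a random launch velocity and clears the inventory.
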(event `self.Pit.OnComponentBeginOverlap`
  (params (OverlappedComponent :type "PrimitiveComponent Object Reference") (OtherActor :type "Actor Object Reference") (OtherComp :type "PrimitiveComponent Object Reference") (OtherBodyIndex :type Integer) (bFromSweep :type Boolean) (SweepResult :type "HitResult Structure (by ref)"))
  ;[0 0 0] As long as colliding object is an tagged as an ingredient
  (if (`ActorComponent.ComponentHasTag` (`Actor.RootComponent` OtherActor) "Ingredient")
    (bind _asitem (cast `/Game/Blueprints/Potions/Item` OtherActor))
    (`self.AddItem` _asitem)
    (`self.DeleteItem` _asitem)
    (`self.CheckPotionList`)))

(fn `AddItem`
  (params (Item :type "/Game/Blueprints/Potions/Item Object Reference"))
  ;[0 0 0] Add item to our current inventory
  (`GameplayStatics.PlaySound2D` "/Game/Audio/Water_Splash-small_1.Water_Splash-small_1" 1.0 1.0 0.0 null null)
  (`BlueprintMapLibrary.Map_Add` (`self.Inventory`) (`/Game/Blueprints/Potions/Item.ItemName` (`local.Item`)) (+ (`BlueprintMapLibrary.Map_Find` (`self.Inventory`) (`/Game/Blueprints/Potions/Item.ItemName` Item)) 1)))

(fn `CanCraftPotion`
  (params (Array :type "Array of String"))
  (returns (returnValue :type Boolean))
  (locals (ItemCount :type Integer))
  (set `local.ItemCount` 0)
  ;[0 0 0] Iterate over recipe items and check if they are in inventory
  (for _array_element (`local.Array`)
    (if (`BlueprintMapLibrary.Map_Contains` (`self.Inventory`) _array_element)
      (`/Engine/EditorBlueprintResources/StandardMacros.IncrementInt` (`local.ItemCount`))
      (else
        (break))))
  ;[0 0 0] True if we have at least 1 of each type
  (return (>= (`local.ItemCount`) (`KismetArrayLibrary.Array_Length` (`local.Array`)))))

(fn `CheckPotionList`
  (bind _returnvalue (`KismetMathLibrary.RandomFloatInRange` 10.0 50.0))
  ;[0 0 0] Use our makeshift "2D Array" to get ingredients from our struct of recipes and check to see if we have all of the ingredients to craft the potion
  (for _array_element (`self.Recipes`)
    (bind (_ingredients _output) (break `/Game/Blueprints/Recipe` _array_element))
    (bind _returnvalue_2 (`self.CanCraftPotion` _ingredients))
    ;[0 0 0] If we have all items, spawn our potion with a bit of a bounce
    (if _returnvalue_2
      (`GameplayStatics.PlaySound2D` "/Game/Audio/Bottle__Cork_Cork_Pop_And_Slosh__Foley.Bottle__Cork_Cork_Pop_And_Slosh__Foley" 1.0 1.0 0.0 null null)
      (bind _returnvalue_3 (`|SpawnActorFromClass` _output (`SceneComponent.K2_GetComponentToWorld` (`self.SpawnLocation`)) "Undefined" "OverrideRootScale" null null))
      (set `MovementComponent.Velocity` (* (`KismetMathLibrary.MakeVector` _returnvalue _returnvalue _returnvalue) 100.0) (`/Game/Blueprints/Potions/Item.ProjectileMovement` _returnvalue_3))
      (`BlueprintMapLibrary.Map_Clear` (`self.Inventory`)) ; Clear our inventory after potion is made
    )))

(fn `DeleteItem`
  (params (Item :type "Actor Object Reference"))
  (`self.K2_DestroyActor` Item))

(fn `UserConstructionScript`)